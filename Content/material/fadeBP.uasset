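; Blueprint that alternates a Sphere's material FadeColor between overbright red and green about once per second.
; Tick branches on ToRed, recreates a dynamic material instance each frame to set the color, then flips the flag after a Delay.
; Despite the name, the switch has no interpolation in Blueprint.
; A disconnected chain holds an unused gradual fade that steps R and G counters and reverses at 255.
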(event EventTick
  (params (DeltaSeconds :type Float%20%28single-precision%29))
  (if (Variables|Default|GettoRed)
    (bind _returnvalue (Rendering|Material|CreateDynamicMaterialInstance (Variables|Default|GetSphere) 0 0 "None" :!class /Script/Engine.PrimitiveComponent))
    (Rendering|Material|SetVectorParameterValue _returnvalue "FadeColor" "(R=255.000000,G=0.000000,B=0.000000,A=1.000000)" :!class /Script/Engine.MaterialInstanceDynamic)
    (Utilities|FlowControl|Delay 1.0)
    (Variables|Default|SettoRed false)
    (else
      (bind _returnvalue_2 (Rendering|Material|CreateDynamicMaterialInstance (Variables|Default|GetSphere) 0 0 "None" :!class /Script/Engine.PrimitiveComponent))
      (Rendering|Material|SetVectorParameterValue _returnvalue_2 "FadeColor" "(R=0.000000,G=255.000000,B=0.000000,A=1.000000)" :!class /Script/Engine.MaterialInstanceDynamic)
      (Utilities|FlowControl|Delay 1.0)
      (Variables|Default|SettoRed true))))

(fn ConstructionScript)