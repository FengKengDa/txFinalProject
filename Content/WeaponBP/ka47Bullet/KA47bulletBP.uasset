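; KA47 bullet actor that damages hookerCHA characters on impact.
; A hit on its static mesh casts the other actor to hookerCHA and subtracts a fixed amount from its Life.
; When Life runs out, it destroys that character and spawns a KA47_Pickable weapon drop at the bullet's own transform.
; The bullet then destroys itself after a zero-length delay.
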(event OnComponentHit(StaticMesh)
  (params (HitComponent :type Primitive%20Component%20Object%20Reference) (OtherActor :type Actor%20Object%20Reference) (OtherComp :type Primitive%20Component%20Object%20Reference) (NormalImpulse :type Vector :default "0, 0, 0") (Hit :type Hit%20Result%20Structure%20%28by%20ref%29))
  (bind _ashooker_cha (Utilities|Casting|CastTohookerCHA OtherActor)
    (:then
      (Variables|/Game/AI/Hooker/hookerCHA.hookerCHA_C|SetLife _ashooker_cha (- (Variables|/Game/AI/Hooker/hookerCHA.hookerCHA_C|GetLife _ashooker_cha) 5))
      (if (<= (Variables|/Game/AI/Hooker/hookerCHA.hookerCHA_C|GetLife _ashooker_cha) 0)
        (Actor|DestroyActor OtherActor)
        (Game|SpawnActorfromClass "/Game/FPS_Weapon_Bundle/Weapons/Meshes/Ka47/KA47_Pickable.KA47_Pickable_C" (Transformation|GetActorTransform) "Undefined" 0 0)))
    (:CastFailed
      _))
  (Utilities|FlowControl|Delay 0.0)
  (Actor|DestroyActor))

(fn ConstructionScript)