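; HookerBP is an AI enemy Blueprint with pawn sensing and a Life value, left mostly unwired.
; Seeing a ThirdPersonCharacter stores the cast result and prints a debug greeting, while the AIMoveTo chase toward it is disconnected.
; The capsule hit event is empty: the bullet damage and destroy-at-zero-Life logic is disconnected, with a note that damage now lives in the bullet.
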(event OnSeePawn(PawnSensing)
  (params (Pawn :type Pawn%20Object%20Reference))
  ;[1 1 1] 追踪
  (bind _asthird_person_character (Utilities|Casting|CastToThirdPersonCharacter Pawn))
  (Development|PrintString "Hello"))

(event OnComponentHit(Capsule)
  (params (HitComponent :type Primitive%20Component%20Object%20Reference) (OtherActor :type Actor%20Object%20Reference) (OtherComp :type Primitive%20Component%20Object%20Reference) (NormalImpulse :type Vector :default "0, 0, 0") (Hit :type Hit%20Result%20Structure%20%28by%20ref%29))
  ;[1 1 1] 扣血，这里先禁用，放子弹里
)

(fn ConstructionScript)